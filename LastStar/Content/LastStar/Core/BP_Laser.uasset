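; BP_Laser is a laser shot actor that deals damage to whatever it hits and then destroys itself.
; On spawn it replaces its tags with its owner's first tag.
; Hit damage always credits player controller 0 as instigator, and Tick destroys the laser once its Cylinder leaves a fixed world X range on either side of the origin.
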(event `self.ReceiveBeginPlay`
  (set `self.Tags` (`|MakeArray` (`|GetArrayItem` (`Actor.Tags` (`self.GetOwner`))))))

(event `self.ReceiveHit`
  (params (MyComp :type "PrimitiveComponent Object Reference") (Other :type "Actor Object Reference") (OtherComp :type "PrimitiveComponent Object Reference") (bSelfMoved :type Boolean) (HitLocation :type "Vector Structure") (HitNormal :type "Vector Structure") (NormalImpulse :type "Vector Structure") (Hit :type "HitResult Structure (by ref)"))
  (`GameplayStatics.ApplyDamage` Other 1.0 (`GameplayStatics.GetPlayerController` 0) self)
  (`self.Destroy`))

(event `self.ReceiveTick`
  (params (DeltaSeconds :type "Float (single-precision)"))
  (bind _returnvalue_x (`KismetMathLibrary.BreakVector` (`SceneComponent.K2_GetComponentLocation` (`self.Cylinder`))))
  (if (or (> _returnvalue_x 2000.0) (< _returnvalue_x -2000.0))
    (`self.Destroy`)))

(fn `Destroy`
  (`self.K2_DestroyActor`))

(fn `UserConstructionScript`)