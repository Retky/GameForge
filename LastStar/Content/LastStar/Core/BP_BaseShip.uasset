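; BP_BaseShip is a base ship actor that provides shooting, damage and death.
; ColorSetUp creates a dynamic material on the ship mesh, which DamageFlash briefly recolors with emissive glow on a hit.
; AnyDamage ignores causers sharing the ship's first tag, otherwise flashes, reduces Life and destroys the ship at zero or below.
; Shoot spawns an owned BP_Laser at the LaserSpawn transform.
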(event `ColorSetUp`
  (bind _returnvalue (`PrimitiveComponent.CreateDynamicMaterialInstance` (`self.SpaceShip`) 0 null "None"))
  (bind _output_get (set `self.BaseColor` _returnvalue))
  (`MaterialInstanceDynamic.SetVectorParameterValue` _output_get "Color" (`self.Color`)))

(event `self.ReceiveAnyDamage`
  (params (Damage :type "Float (single-precision)") (DamageType :type "DamageType Object Reference") (InstigatedBy :type "Controller Object Reference") (DamageCauser :type "Actor Object Reference"))
  (if (not (`self.ActorHasTag` DamageCauser (`|GetArrayItem` (`self.Tags`))))
    (`self.Damage Flash`)
    (set `self.Life` (`KismetMathLibrary.FTrunc` (- (`self.Life`) Damage)))
    (`self.Die?`)))

(event `Damage Flash`
  (bind _basecolor (`self.BaseColor`))
  (bind _flashcolor (`self.FlashColor`))
  (`MaterialInstanceDynamic.SetVectorParameterValue` _basecolor "Color" _flashcolor)
  (`MaterialInstanceDynamic.SetVectorParameterValue` _basecolor "Emissive Color" _flashcolor)
  (`MaterialInstanceDynamic.SetScalarParameterValue` _basecolor "Emissive Multipier" 1.0)
  (`KismetSystemLibrary.Delay` 0.1)
  (`MaterialInstanceDynamic.SetVectorParameterValue` _basecolor "Color" (`self.Color`))
  (`MaterialInstanceDynamic.SetVectorParameterValue` :`self` _basecolor :`ParameterName` "Emissive Color")
  (`MaterialInstanceDynamic.SetScalarParameterValue` _basecolor "Emissive Multipier" 0.0))

(fn `Die?`
  (if (<= (`self.Life`) 0)
    (`self.K2_DestroyActor`)))

(fn `Shoot`
  (`|SpawnActorFromClass` "/Game/LastStar/Core/BP_Laser.BP_Laser_C" (`SceneComponent.K2_GetComponentToWorld` (`self.LaserSpawn`)) "Undefined" "MultiplyWithRoot" self null))

(fn `UserConstructionScript`)