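; Player-controlled ship pawn that moves and shoots through Enhanced Input.
; BeginPlay calls ColorSetUp, then adds the ship's input mapping context to the local player.
; Move input drives sideways and forward/back movement relative to control rotation, with forward/back gated by the Box component's world X to keep the ship within a fixed band.
; Shoot input calls Shoot, whose logic, like ColorSetUp's, is defined outside these graphs.
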(event `self.ReceiveBeginPlay`
  (`self.ColorSetUp`)
  ;[0.5051 0.7497 1] Movement
  (bind _asplayer_controller (cast `PlayerController` (`self.GetController`)))
  (bind _returnvalue (pcsubsystem `EnhancedInputLocalPlayerSubsystem` _asplayer_controller))
  (`/Engine/EditorBlueprintResources/StandardMacros.IsValid` _returnvalue
    (:`Is Valid`
      (`EnhancedInputSubsystemInterface.AddMappingContext` _returnvalue "/Game/LastStar/Input/IMC_PlayerShip.IMC_PlayerShip" 0 (struct)))))

(event `EnhancedInput|/Game/LastStar/Input/IA_Move`
  (params (ActionValue :type "Vector2D Structure") (ElapsedSeconds :type "Float (double-precision)") (TriggeredSeconds :type "Float (double-precision)") (InputAction :type "InputAction Object Reference" :default "/Game/LastStar/Input/IA_Move.IA_Move"))
  (bind (_returnvalue_roll _returnvalue_pitch _returnvalue_yaw) (`KismetMathLibrary.BreakRotator` (`self.GetControlRotation`)))
  (bind (_returnvalue_roll_2 _returnvalue_pitch_2 _returnvalue_yaw_2) (`KismetMathLibrary.BreakRotator` (`self.GetControlRotation`)))
  (bind _returnvalue_x (`KismetMathLibrary.BreakVector` (`SceneComponent.K2_GetComponentLocation` (`self.Box`))))
  ;[0.5051 0.7497 1] Movement
  (:`Triggered`
    (`self.AddMovementInput` (`KismetMathLibrary.GetRightVector` (`KismetMathLibrary.MakeRotator` _returnvalue_roll 0.0 _returnvalue_yaw)) ActionValue_X)
    (if (and (or (> ActionValue_Y 0.0) (<= _returnvalue_x 80.0)) (or (< ActionValue_Y 0.0) (>= _returnvalue_x -500.0)))
      (`self.AddMovementInput` (`KismetMathLibrary.GetForwardVector` (`KismetMathLibrary.MakeRotator` 0.0 0.0 _returnvalue_yaw_2)) ActionValue_Y))))

(event `EnhancedInput|/Game/LastStar/Input/IA_Shoot`
  (params (ActionValue :type Boolean) (ElapsedSeconds :type "Float (double-precision)") (TriggeredSeconds :type "Float (double-precision)") (InputAction :type "InputAction Object Reference" :default "/Game/LastStar/Input/IA_Shoot.IA_Shoot"))
  (:`Triggered`
    (`self.Shoot`)))

(fn `UserConstructionScript`
  (`parent.UserConstructionScript`))