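; BP_BaseShip is a ship Blueprint for LastStar that fires a laser and takes damage.
; Two seconds after BeginPlay it fires once, spawning a BP_Laser at the LaserSpawn transform with itself as owner.
; AnyDamage treats a causer carrying the ship's first tag as a friend and ignores the hit.
; Other damage reduces Life, and the ship is destroyed at zero or below.
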(event `self.ReceiveBeginPlay`
  (`KismetSystemLibrary.Delay` 2.0)
  (`self.Shot`))

(event `self.ReceiveAnyDamage`
  (params (Damage :type "Float (single-precision)") (DamageType :type "DamageType Object Reference") (InstigatedBy :type "Controller Object Reference") (DamageCauser :type "Actor Object Reference"))
  (if (`self.ActorHasTag` DamageCauser (`|GetArrayItem` (`self.Tags`)))
    (`KismetSystemLibrary.PrintString` "Friend")
    (else
      (`KismetSystemLibrary.PrintString` "Enemy")
      (set `self.Life` (`KismetMathLibrary.FTrunc` (- (`self.Life`) Damage)))
      (`self.Die?`))))

(fn `Die?`
  (if (<= (`self.Life`) 0)
    (`self.K2_DestroyActor`)))

(fn `Shot`
  (`|SpawnActorFromClass` "/Game/LastStar/BP_Laser.BP_Laser_C" (`SceneComponent.K2_GetComponentToWorld` (`self.LaserSpawn`)) "Undefined" "MultiplyWithRoot" self null))

(fn `UserConstructionScript`)