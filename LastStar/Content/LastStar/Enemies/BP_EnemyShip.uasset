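; BP_EnemyShip is an enemy ship that flies in along a spline, fires, then flies out and destroys itself.
; Timelines drive position and rotation by spline distance along PathIn and PathOut.
; A delayed loop calls Shoot while Fire is set, starting at spawn and stopping on arrival.
; ShootTime then pauses, runs a short burst at a fixed interval, pauses again and triggers the exit.
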(event `self.ReceiveBeginPlay`
  (`self.ColorSetUp`)
  (`self.MoveIn`)
  (`self.ShootEvent`))

(event `MoveIn`
  (bind _spline (`/Game/LastStar/Enemies/BP_SplinePath.Spline` (`self.PathIn`)))
  (`TimelineComponent.SetPlayRate` (`self.Move T`) (/ 1.0 2.0))
  (bind (_direction _movetrack) (`Timeline|Move T`)
    (:`Update`
      (bind _returnvalue (`KismetMathLibrary.Lerp` 0.0 (`SplineComponent.GetSplineLength` _spline) _movetrack))
      (`self.K2_SetActorTransform` (`KismetMathLibrary.MakeTransform` (`SplineComponent.GetLocationAtDistanceAlongSpline` _spline _returnvalue "World") (`SplineComponent.GetRotationAtDistanceAlongSpline` _spline _returnvalue "World"))))
    (:`Finished`
      (set `self.bFire` false)
      (`self.ShootTime`))))

(event `MoveOut`
  (bind _spline (`/Game/LastStar/Enemies/BP_SplinePath.Spline` (`self.PathOut`)))
  (`TimelineComponent.SetPlayRate` (`self.Move Out T`) (/ 1.0 2.5))
  (bind (_direction _movetrack) (`Timeline|Move Out T`)
    (:`Update`
      (bind _returnvalue (`KismetMathLibrary.Lerp` 0.0 (`SplineComponent.GetSplineLength` _spline) _movetrack))
      (`self.K2_SetActorTransform` (`KismetMathLibrary.MakeTransform` (`SplineComponent.GetLocationAtDistanceAlongSpline` _spline _returnvalue "World") (`SplineComponent.GetRotationAtDistanceAlongSpline` _spline _returnvalue "World"))))
    (:`Finished`
      (`self.K2_DestroyActor`))))

(event `ShootEvent`
  (`KismetSystemLibrary.Delay` (`self.ShootInterval`) :!label _label)
  (`self.Shoot`)
  (while (`self.bFire`)
    (goto _label)))

(event `ShootTime`
  (`KismetSystemLibrary.Delay` 1.5)
  (set `self.bFire` true)
  (set `self.ShootInterval` 0.3)
  (`self.ShootEvent`)
  (`KismetSystemLibrary.Delay` 0.8)
  (set `self.bFire` false)
  (`KismetSystemLibrary.Delay` 1.5)
  (`self.MoveOut`))

(fn `UserConstructionScript`
  (`parent.UserConstructionScript`))