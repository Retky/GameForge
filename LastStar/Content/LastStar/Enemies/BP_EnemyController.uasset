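; Enemy wave spawner for LastStar that starts a new wave on BeginPlay and shortly after all attached enemy ships are gone.
; Each wave spawns mirrored left/right ship pairs in a grid, giving each ship its own in and out spline paths.
; Attached actors serve as the live-enemy count.
; Integer-division modulo cycles pair count up to MaxEnemies, with each completed cycle raising life, stand time and points.
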(event `self.ReceiveBeginPlay`
  (set `self.Pawn` (`GameplayStatics.GetPlayerPawn` 0))
  (`self.WaveController`))

(event `self.ReceiveTick`
  (params (DeltaSeconds :type "Float (single-precision)"))
  (if (and (<= (`KismetArrayLibrary.Array_Length` (`self.GetAttachedActors` true)) 0) (not (`self.Summoning`)))
    (set `self.Summoning` true)
    (`KismetSystemLibrary.Delay` 1.8)
    (`self.WaveController`)))

(event `WaveController`
  (bind _enemycolumns (`self.EnemyColumns`))
  (bind _maxenemies (`self.MaxEnemies`))
  (bind _waves (`self.Waves`))
  (bind _returnvalue (/ _waves _maxenemies))
  (if (`KismetSystemLibrary.IsValid` (`self.Pawn`))
    (for _index (range (+ (- _waves (* _returnvalue _maxenemies)) 1))
      (bind _returnvalue_2 (/ _index _enemycolumns))
      (bind _returnvalue_3 (- _index (* _returnvalue_2 _enemycolumns)))
      (bind _returnvalue_4 (* _returnvalue_2 150))
      (`self.SummonEnemy` (`self.ModPosition` _returnvalue_3 (`KismetMathLibrary.MakeTransform` (`KismetMathLibrary.MakeVector` (+ _returnvalue_4 (.x (.location (`self.Position Left`)))) (.y (.location (`self.Position Left`))) (.z (.location (`self.Position Left`)))) (.rotation (`self.Position Left`)) (.scale (`self.Position Left`)))) (`self.ModPosition` (* _returnvalue_3 -1) (`KismetMathLibrary.MakeTransform` (`KismetMathLibrary.MakeVector` (+ _returnvalue_4 (.x (.location (`self.Position Rigth`)))) (.y (.location (`self.Position Rigth`))) (.z (.location (`self.Position Rigth`)))) (.rotation (`self.Position Rigth`)) (.scale (`self.Position Rigth`)))) (+ _returnvalue 1) (+ (* 1.0 _returnvalue) 4.0) (+ (* _returnvalue 10) 10)))
    (`/Engine/EditorBlueprintResources/StandardMacros.IncrementInt` _waves)))

(fn `ModPosition`
  (params (Multiply :type Integer) (BasePosition :type "Transform Structure"))
  (returns (NewPosition :type "Transform Structure"))
  (return (`KismetMathLibrary.MakeTransform` (+ (`KismetMathLibrary.MakeVector` 0.0 (* Multiply 150.0)) (.location BasePosition)) (.rotation BasePosition) (.scale BasePosition))))

(fn `SummonEnemy`
  (params (PositionLeft :type "Transform Structure") (PositionRigth :type "Transform Structure") (Life :type Integer) (StandTime :type "Float (double-precision)") (Points :type Integer))
  (bind _returnvalue (`|SpawnActorFromClass` "/Game/LastStar/Enemies/BP_SplinePath_In1.BP_SplinePath_In1_C" PositionLeft "Undefined" "MultiplyWithRoot" null null))
  (bind _returnvalue_2 (`|SpawnActorFromClass` "/Game/LastStar/Enemies/BP_SplinePath_Out1.BP_SplinePath_Out1_C" PositionLeft "Undefined" "MultiplyWithRoot" null null))
  (bind _returnvalue_3 (`|SpawnActorFromClass` "/Game/LastStar/Enemies/BP_EnemyShip.BP_EnemyShip_C" (`KismetMathLibrary.MakeTransform` (+ (.location PositionLeft) (-500.0 1000.0 0.0)) (.rotation PositionLeft) (.scale PositionLeft)) "Undefined" "MultiplyWithRoot" null _returnvalue _returnvalue_2 StandTime Points Life null))
  (`self.K2_AttachToActor` _returnvalue_3 self "Enemies" "KeepRelative" "KeepRelative" "KeepRelative" true)
  (bind _returnvalue_4 (`|SpawnActorFromClass` "/Game/LastStar/Enemies/BP_SplinePath_In2.BP_SplinePath_In2_C" PositionRigth "Undefined" "MultiplyWithRoot" null null))
  (bind _returnvalue_5 (`|SpawnActorFromClass` "/Game/LastStar/Enemies/BP_SplinePath_Out2.BP_SplinePath_Out2_C" PositionRigth "Undefined" "MultiplyWithRoot" null null))
  (bind _returnvalue_6 (`|SpawnActorFromClass` "/Game/LastStar/Enemies/BP_EnemyShip.BP_EnemyShip_C" (`KismetMathLibrary.MakeTransform` (+ (.location PositionRigth) (-500.0 -1000.0 0.0)) (.rotation PositionRigth) (.scale PositionRigth)) "Undefined" "MultiplyWithRoot" null _returnvalue_4 _returnvalue_5 StandTime Points Life null))
  (`self.K2_AttachToActor` _returnvalue_6 self "Enemies" "KeepRelative" "KeepRelative" "KeepRelative" true)
  (set `self.Summoning` false))

(fn `UserConstructionScript`)